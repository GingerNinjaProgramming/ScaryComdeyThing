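; BP_DungeonHandler is an early-stage dungeon generator that places the starting room of a room-based dungeon.
; On BeginPlay it spawns BP_DungeonRoom1 at its root transform and collects the children of that room's ExitsFolder into ExitsList.
; SpawnNextRoom is an unfinished stub that nothing here calls: it removes a random exit from the list and clears SelectedExitPoint without spawning a room.
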(event Custom|SpawnStartRoom
  ;[0.000146 0.4662 0.5052 0.5] Spawn Start Room
  (bind _returnvalue (Game|SpawnActorfromClass "/Game/Blueprints/Dungeon/Rooms/BP_DungeonRoom-1.BP_DungeonRoom-1_C" (Transformation|GetWorldTransform (Variables|Default|GetDefaultSceneRoot)) "Undefined" "MultiplyWithRoot" 0 0))
  (Utilities|Array|AppendArray (Variables|Default|GetExitsList) (Components|GetChildrenComponents (Variables|/Game/Blueprints/Dungeon/BP_MasterRoom.BP_MasterRoom_C|GetExitsFolder _returnvalue) false)))

(event Custom|SpawnNextRoom
  (CallFunction|GetRandomElementandRemove 0 (Variables|Default|GetExitsList))
  (Variables|Default|SetSelectedExitPoint 0))

(event EventBeginPlay
  (CallFunction|SpawnStartRoom))

(fn ConstructionScript)